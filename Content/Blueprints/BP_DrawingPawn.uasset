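; BP_DrawingPawn is a pawn that lets the player paint on BP_Canvas actors with the mouse.
; While the left button is held, Tick traces under the cursor with complex collision and converts the hit to a UV via FindCollisionUV.
; DrawBrush draws a dynamic M_Brush material at that UV onto the canvas's render target, centred by brush size.
; Setter functions change the brush texture and size.
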(event EventBeginPlay
  (Utilities|FlowControl|Sequence
    (:then_0
      (Variables|/Script/Engine.PlayerController|SetbShowMouseCursor (Game|GetPlayerController 0) true))
    (:then_1
      (bind _returnvalue (Rendering|Material|CreateDynamicMaterialInstance "/Game/Materials/M_Brush.M_Brush" "None" "None" :!class /Script/Engine.KismetMaterialLibrary))
      (Variables|Default|SetMI_Brush _returnvalue))))

(event EventTick
  (params (DeltaSeconds :type Float%20%28single-precision%29))
  (bind _returnvalue (Game|GetPlayerController 0))
  (bind (_hitresult _returnvalue_2) (Game|Player|GetHitResultUnderCursorbyChannel _returnvalue "TraceTypeQuery1" true))
  (bind (_bblockinghit _binitialoverlap _time _distance _location _impactpoint _normal _impactnormal _physmat _hitactor _hitcomponent _hitbonename _hititem _elementindex _faceindex _tracestart _traceend) (Collision|BreakHitResult _hitresult))
  (if (Variables|Default|GetDrawing)
    (if _returnvalue_2
      (bind _asbp_canvas (Utilities|Casting|CastToBP_Canvas _hitactor))
      (bind _outhit (Collision|LineTraceByChannel _tracestart _traceend "TraceTypeQuery1" true 0 "None"))
      (CallFunction|DrawBrush (.UV (Class|GameplayStatics|FindCollisionUV _outhit)) (Variables|/Game/Blueprints/BP_Canvas.BP_Canvas_C|GetRenderTarget _asbp_canvas)))))

(event Input|MouseEvents|LeftMouseButton
  (params (Key :type Key%20Structure :default "None"))
  (:Pressed
    (Variables|Default|SetDrawing true))
  (:Released
    (Variables|Default|SetDrawing false)))

(fn ConstructionScript)

(fn DrawBrush
  (params (Location :type Vector%202D%20Structure) (TargetCanvas :type Texture%20Render%20Target%202D%20Object%20Reference))
  (bind _brushsize (Variables|Default|GetBrushSize))
  (bind (_canvas _size _context) (Rendering|BeginDrawCanvastoRenderTarget TargetCanvas))
  (Canvas|DrawMaterial :self _canvas :RenderMaterial (Variables|Default|GetMI_Brush) :ScreenPosition (- (* _size Location) (/ _brushsize 2.0)) :ScreenSize (Math|Vector2D|MakeVector2D _brushsize _brushsize) :CoordinateSize "(X=1.000000,Y=1.000000)" :PivotPoint "(X=0.500000,Y=0.500000)")
  (Rendering|EndDrawCanvastoRenderTarget _context))

(fn SetBrushTexture
  (params (NewTexture :type Texture%202D%20Object%20Reference))
  (if (!= NewTexture (Variables|Default|GetBrushTexture))
    (bind _output_get (Variables|Default|SetBrushTexture NewTexture))
    (Rendering|Material|SetTextureParameterValue (Variables|Default|GetMI_Brush) "BrushTexture" _output_get)))

(fn SetBrushSize
  (params (NewSize :type Float%20%28single-precision%29))
  (if (!= NewSize (Variables|Default|GetBrushSize))
    (Variables|Default|SetBrushSize NewSize)))