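; Default player controller that manages the local player's UI widgets for a word-choosing game with a leaderboard.
; The Quit input toggles an in-game menu, while controller events show candidate words, hide them once a word is chosen, and display or clear the leaderboard around game restarts.
; Each widget is created lazily on first use, cached, and then added to or removed from the viewport.
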(event EventOnReceiveCandidateWords
  (params (CandidateWords :type Array%20of%20Strings))
  (Utilities|IsValid (Variables|Default|GetChooseWordWidget)
    (:Is%20Valid
      (if (UserInterface|Viewport|IsinViewport (Variables|Default|GetChooseWordWidget))
        _
        (else
          (UserInterface|Viewport|AddtoViewport (Variables|Default|GetChooseWordWidget) 0 :!label _label))))
    (:Is%20Not%20Valid
      (bind _returnvalue (UserInterface|CreateWidget "/Game/UI/InGame/BP_Widget_ChooseWord.BP_Widget_ChooseWord_C" self))
      (Variables|Default|SetChooseWordWidget _returnvalue)
      (goto _label)))
  (Default|SetCandidateWords (Variables|Default|GetChooseWordWidget) CandidateWords))

(event EventOnWordChosen
  (bind _choosewordwidget (Variables|Default|GetChooseWordWidget))
  (Utilities|IsValid _choosewordwidget
    (:Is%20Valid
      (if (UserInterface|Viewport|IsinViewport _choosewordwidget)
        (Widget|RemovefromParent _choosewordwidget)))))

(event EventOnReceiveLeaderboardData
  (params (NameArray :type Array%20of%20Strings) (ScoreArray :type Array%20of%20Integers))
  (Utilities|IsValid (Variables|Default|GetLeaderboardWidget)
    (:Is%20Valid
      _)
    (:Is%20Not%20Valid
      (bind _returnvalue (UserInterface|CreateWidget "/Game/UI/InGame/BP_Widget_Leaderboard.BP_Widget_Leaderboard_C" self))
      (Variables|Default|SetLeaderboardWidget _returnvalue)))
  (UserInterface|Viewport|AddtoViewport (Variables|Default|GetLeaderboardWidget) 0)
  (Default|SetupLeaderboard (Variables|Default|GetLeaderboardWidget) NameArray ScoreArray))

(event EventOnReceiveGameRestart
  (bind _leaderboardwidget (Variables|Default|GetLeaderboardWidget))
  (Utilities|IsValid _leaderboardwidget
    (:Is%20Valid
      (if (UserInterface|Viewport|IsinViewport _leaderboardwidget)
        (Widget|RemovefromParent _leaderboardwidget)))))

(event Input|ActionEvents|InputActionQuit
  (params (Key :type Key%20Structure :default "None"))
  (:Released
    (Utilities|IsValid (Variables|Default|GetInGameMenuWidget)
      (:Is%20Valid
        _)
      (:Is%20Not%20Valid
        (bind _returnvalue (UserInterface|CreateWidget "/Game/UI/InGame/BP_Widget_InGameMenu.BP_Widget_InGameMenu_C" self))
        (bind _output_get (Variables|Default|SetInGameMenuWidget _returnvalue))))
    (if (UserInterface|Viewport|IsinViewport (Variables|Default|GetInGameMenuWidget))
      (Widget|RemovefromParent _output_get)
      (else
        (UserInterface|Viewport|AddtoViewport _output_get 0)))))

(fn ConstructionScript)